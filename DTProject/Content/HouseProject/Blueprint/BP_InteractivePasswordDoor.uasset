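; BP_InteractivePasswordDoor is a door that swings open when a controlled Pawn overlaps its collision, and swings back when it leaves.
; A dot product of the actor's right vector and the Pawn's offset picks the sign of the target yaw, so swing direction follows the approach side.
; A Timeline lerps the relative yaw from BaseYaw to that signed DeltaYaw, reversing on end overlap.
; Despite the name, it contains no password logic.
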(event `self.CollisionComp.OnComponentBeginOverlap`
  (params (OverlappedComponent :type "PrimitiveComponent Object Reference") (OtherActor :type "Actor Object Reference") (OtherComp :type "PrimitiveComponent Object Reference") (OtherBodyIndex :type Integer) (bFromSweep :type Boolean) (SweepResult :type "HitResult Structure (by ref)"))
  (bind _aspawn (cast `Pawn` OtherActor))
  (if (`Pawn.IsControlled` _aspawn)
    (bind _playerlocationvalue (`self.Get Enter Direction` (`self.CollisionComp`) OtherActor))
    (bind (_direction _rate) (`Timeline|Timeline` :!label _label)
      (:`Update`
        (bind _door_rotaor (`self.Set Door Rotator` _playerlocationvalue _rate))
        (`SceneComponent.K2_SetRelativeRotation` (`self.Door`) _door_rotaor false false)))))

(event `self.CollisionComp.OnComponentEndOverlap`
  (params (OverlappedComponent :type "PrimitiveComponent Object Reference") (OtherActor :type "Actor Object Reference") (OtherComp :type "PrimitiveComponent Object Reference") (OtherBodyIndex :type Integer))
  (bind _aspawn (cast `Pawn` OtherActor))
  (if (`Pawn.IsControlled` _aspawn)
    (goto _label :!via `Reverse`)))

(fn `Get Enter Direction`
  (params (OverlapCollision :type "ActorComponent Object Reference") (OverlapPlayer :type "Actor Object Reference"))
  (returns (PlayerLocationValue :type Boolean))
  (return (> (`KismetMathLibrary.Dot_VectorVector` (`self.GetActorRightVector`) (- (`self.K2_GetActorLocation` OverlapPlayer) (`self.K2_GetActorLocation` (`ActorComponent.GetOwner` OverlapCollision)))) 0.0)))

(fn `Set Door Rotator`
  (params (`Enter Direction` :type Boolean) (`Direction Value` :type "Float (double-precision)"))
  (returns (`Door Rotaor` :type "Rotator Structure"))
  (return (`KismetMathLibrary.MakeRotator` 0.0 0.0 (`KismetMathLibrary.Lerp` (`self.BaseYaw`) (* (`self.DeltaYaw`) (`KismetMathLibrary.SelectFloat` -1.0 1.0 `Enter Direction`)) `Direction Value`))))

(fn `UserConstructionScript`
  (`parent.UserConstructionScript`))