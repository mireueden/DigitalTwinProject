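; Interactive warehouse door actor, still unfinished, meant to respond to a controlled pawn entering or leaving its collision component.
; Overlap plays a timeline forward and end overlap reverses it.
; Each update loops over the door array, which lists the third door twice, but only sweeps the actor itself to world origin.
; GetEnterDirection is a stub returning false, and its result is unused.
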(event `self.ReceiveBeginPlay`
  (`parent.ReceiveBeginPlay`)
  (set `self.DoorArr` (`|MakeArray` (`self.WareHouseDoor1`) (`self.WareHouseDoor2`) (`self.WareHouseDoor3`) (`self.WareHouseDoor3`))))

(event `self.CollisionComp.OnComponentBeginOverlap`
  (params (OverlappedComponent :type "PrimitiveComponent Object Reference") (OtherActor :type "Actor Object Reference") (OtherComp :type "PrimitiveComponent Object Reference") (OtherBodyIndex :type Integer) (bFromSweep :type Boolean) (SweepResult :type "HitResult Structure (by ref)"))
  (bind _aspawn (cast `Pawn` OtherActor))
  (if (`Pawn.IsControlled` _aspawn)
    (`self.Get Enter Direction` (`self.CollisionComp`) OtherActor)
    (`Timeline|Timeline` :!label _label
      (:`Update`
        (for _ (`self.DoorArr`)
          (`self.K2_SetActorLocation` (0.0 0.0 0.0) true))))))

(event `self.CollisionComp.OnComponentEndOverlap`
  (params (OverlappedComponent :type "PrimitiveComponent Object Reference") (OtherActor :type "Actor Object Reference") (OtherComp :type "PrimitiveComponent Object Reference") (OtherBodyIndex :type Integer))
  (bind _aspawn (cast `Pawn` OtherActor))
  (if (`Pawn.IsControlled` _aspawn)
    (goto _label :!via `Reverse`)))

(fn `Get Enter Direction`
  (params (OverlapCollision :type "ActorComponent Object Reference") (OverlapPlayer :type "Actor Object Reference"))
  (returns (PlayerLocationValue :type Boolean))
  (return false))

(fn `UserConstructionScript`
  (`parent.UserConstructionScript`))