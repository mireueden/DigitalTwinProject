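; First-person player character that lets the player interact with house objects such as microwaves, lamps, light controllers and the warehouse checker.
; Each Tick it line-traces from the camera with debug drawing and stores the hit interactive actor and its data-asset type.
; Pressing E switches on that type, toggling a lamp's point light directly or asking the project GameMode to show or hide UI panels.
; Overlap events restrict opening the warehouse order list to players inside the checker.
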(event `self.ReceiveActorBeginOverlap`
  (params (OtherActor :type "Actor Object Reference"))
  (cast `/Game/HouseProject/Blueprint/BP_InteractiveWareHouseChecker` OtherActor)
  (set `self.bIsCheckerOverlap` true))

(event `self.ReceiveActorEndOverlap`
  (params (OtherActor :type "Actor Object Reference"))
  (cast `/Game/HouseProject/Blueprint/BP_InteractiveWareHouseChecker` OtherActor)
  (set `self.bIsCheckerOverlap` false))

(event `self.ReceiveBeginPlay`
  (bind _asbp_project_game_mode (cast `/Game/HouseProject/GameMode/BP_ProjectGameMode` (`GameplayStatics.GetGameMode`)))
  (set `self.ProjectGameMode` _asbp_project_game_mode))

(event `self.ReceiveTick`
  (params (DeltaSeconds :type "Float (single-precision)"))
  (bind _firstpersoncameracomponent (`self.FirstPersonCameraComponent`))
  (bind _returnvalue (`SceneComponent.K2_GetComponentLocation` _firstpersoncameracomponent))
  (bind _outhit (`KismetSystemLibrary.LineTraceSingle` :`Start` _returnvalue :`End` (+ _returnvalue (* (`SceneComponent.GetForwardVector` _firstpersoncameracomponent) 1000.0)) :`TraceChannel` "TraceTypeQuery1" :`DrawDebugType` "ForDuration" :`DrawTime` 0.1))
  (bind _output_get (set `self.CheckActor` (`.HitActor` (`GameplayStatics.BreakHitResult` _outhit))))
  (bind _asinteractive_actor_base (cast `InteractiveActorBase` _output_get))
  (set `self.CheckActorType` (`ObjectDataAsset.Type` (`InteractiveComponentBase.DataAssetInstance` (`InteractiveActorBase.Component` _asinteractive_actor_base)))))

(event `Key|E`
  (params (Key :type "Key Structure"))
  (bind _projectgamemode (`self.ProjectGameMode`))
  (bind _projectgamemode_2 (`self.ProjectGameMode`))
  (bind _projectgamemode_3 (`self.ProjectGameMode`))
  (bind (_asbp_interactive_light _bsuccess) (cast `/Game/HouseProject/Blueprint/BP_InteractiveLight` (`self.CheckActor`) :!pure true))
  (bind _pointlight (`/Game/HouseProject/Blueprint/BP_InteractiveLight.PointLight` _asbp_interactive_light))
  (:`Pressed`
    (switch `EObjectType` (`self.CheckActorType`)
      (:`Microwave`
        (if (`self.bOpenTurnOnOffPopup`)
          (`/Game/HouseProject/GameMode/BP_ProjectGameMode.Hidden ItemTurnOnOff Event` _projectgamemode)
          (set `self.bOpenTurnOnOffPopup` false)
          (else
            (`/Game/HouseProject/GameMode/BP_ProjectGameMode.Set ItemTurnOnOff Event` _projectgamemode)
            (set `self.bOpenTurnOnOffPopup` true))))
      (:`Lamp`
        (if _bsuccess
          (if (`/Game/HouseProject/Blueprint/BP_InteractiveLight.bIsActorActive` _asbp_interactive_light)
            (set `/Game/HouseProject/Blueprint/BP_InteractiveLight.bIsActorActive` false _asbp_interactive_light)
            (`LightComponent.SetIntensity` _pointlight 0.0)
            (else
              (set `/Game/HouseProject/Blueprint/BP_InteractiveLight.bIsActorActive` true _asbp_interactive_light)
              (`LightComponent.SetIntensity` _pointlight 5000.0)))))
      (:`WareHousChecker`
        (if (`self.bIsCheckerOverlap`)
          (if (`self.bIsCheckerOpen`)
            (`/Game/HouseProject/GameMode/BP_ProjectGameMode.Hidden Order List Event` _projectgamemode_2 :!label _label)
            (set `self.bIsCheckerOpen` false)
            (else
              (`/Game/HouseProject/GameMode/BP_ProjectGameMode.Set Order List Event` _projectgamemode_2)
              (set `self.bIsCheckerOpen` true)))
          (else
            (goto _label))))
      (:`LightController`
        (if (`self.bIsLightListOpen`)
          (`/Game/HouseProject/GameMode/BP_ProjectGameMode.Hidden Light List Event` _projectgamemode_3)
          (set `self.bIsLightListOpen` false)
          (else
            (`/Game/HouseProject/GameMode/BP_ProjectGameMode.Set Light List Event` _projectgamemode_3)
            (set `self.bIsLightListOpen` true)))))))

(fn `UserConstructionScript`)